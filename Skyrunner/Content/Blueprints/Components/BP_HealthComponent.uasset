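; Actor component that tracks health for its owner and broadcasts damage, heal and death events.
; CurrentHealth starts at MaxHealth on BeginPlay.
; DealDamage subtracts health and fires OnDeath at zero or below, otherwise OnDamage, without clamping or guarding against repeated death calls.
; Heal caps health at MaxHealth before firing OnHeal, and IsAlive reports whether health is above zero.
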(event `self.ReceiveBeginPlay`
  (set `self.CurrentHealth` (`self.MaxHealth`)))

(fn `DealDamage`
  (params (Amount :type Integer))
  (bind _output_get (set `self.CurrentHealth` (- (`self.CurrentHealth`) Amount)))
  (if (<= _output_get 0)
    (`self.OnDeath`)
    (else
      (`self.OnDamage`))))

(fn `Heal`
  (params (Amount :type Integer))
  (set `self.CurrentHealth` (+ Amount (`self.CurrentHealth`)))
  (`|ExecutionSequence`
    (:`then_0`
      (if (> (`self.CurrentHealth`) (`self.MaxHealth`))
        (set `self.CurrentHealth` (`self.MaxHealth`))))
    (:`then_1`
      (`self.OnHeal`))))

(fn `IsAlive`
  (returns (IsAlive :type Boolean))
  (return (> (`self.CurrentHealth`) 0)))