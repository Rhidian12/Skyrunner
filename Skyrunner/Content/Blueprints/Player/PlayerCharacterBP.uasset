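; Player character Blueprint that moves from accumulated movement input and carries a hitscan gun.
; On BeginPlay it spawns a BP_HitscanGun, stores it as Gun and attaches it to the GunHand component.
; Each Tick it consumes the movement input vector, clamps it to unit length, and applies a swept, frame-rate-independent world offset scaled by MovementSpeed.
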(event `self.ReceiveBeginPlay`
  (bind _returnvalue (`|SpawnActorFromClass` "/Game/Blueprints/Guns/BP_HitscanGun.BP_HitscanGun_C" (`KismetMathLibrary.MakeTransform` (0.0 0.0 0.0)) "Undefined" "OverrideRootScale" null null))
  (bind _output_get (set `self.Gun` _returnvalue))
  (`self.K2_AttachToComponent` _output_get (`self.GunHand`) "None" "KeepRelative" "KeepRelative" "KeepRelative" true))

(event `self.ReceiveTick`
  (params (DeltaSeconds :type "Float (single-precision)"))
  (bind _returnvalue (`self.ConsumeMovementInputVector`))
  (`self.K2_AddActorWorldOffset` (* (* (`KismetMathLibrary.ClampVectorSize` _returnvalue 0.0 1.0) DeltaSeconds) (`self.MovementSpeed`)) true))

(fn `UserConstructionScript`)