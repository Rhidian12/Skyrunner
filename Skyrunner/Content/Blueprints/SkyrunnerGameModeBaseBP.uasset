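; Skyrunner game mode Blueprint that manages spawn points and the objective cycle.
; On BeginPlay it sorts every BP_Spawn by Type into objective, enemy and any-spawn arrays.
; OnSpawnObjective spawns a random PossibleObjectives class at the world origin, without using those arrays.
; OnObjectiveComplete prints a message, waits five seconds, then calls LoadLevelInstance with the current level name as a restart.
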(event `self.ReceiveBeginPlay`
  (bind _outactors (`GameplayStatics.GetAllActorsOfClass` "/Game/Blueprints/Objectives/BP_Spawn.BP_Spawn_C"))
  (for _array_element _outactors
    (`KismetArrayLibrary.Array_AddUnique` (select `/Game/Blueprints/Objectives/SpawnType` (`/Game/Blueprints/Objectives/BP_Spawn.Type` _array_element) :`NewEnumerator0` (`self.ObjectiveSpawns`) :`NewEnumerator1` (`self.EnemySpawns`) :`NewEnumerator2` (`self.AnySpawns`)) _array_element)))

(event `OnSpawnObjective`
  (`|SpawnActorFromClass` (`KismetArrayLibrary.Array_Random` (`self.PossibleObjectives`)) (`KismetMathLibrary.MakeTransform` (0.0 0.0 0.0)) "AlwaysSpawn" "OverrideRootScale" null null))

(event `OnObjectiveComplete`
  (`KismetSystemLibrary.PrintString` "Objective complete!! Restarting in 5s")
  (`KismetSystemLibrary.Delay` 5.0)
  (bind _returnvalue (`GameplayStatics.GetCurrentLevelName` true))
  (`LevelStreamingDynamic.LoadLevelInstance` _returnvalue (0.0 0.0 0.0) (struct) "" null))

(fn `UserConstructionScript`)