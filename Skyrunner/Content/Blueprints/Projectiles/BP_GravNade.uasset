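; Gravity grenade projectile that launches enemies and leaves an influence actor where it stops.
; When projectile movement stops, it launches every BaseEnemy in the level, with no range check, overriding their velocity.
; Launch direction is the normalized grenade-to-enemy vector with Z scaled by ZMultiplier, multiplied by EnemyLaunchForce.
; It then spawns a scaled-up BP_GravNadeInfluence at its collision location and destroys itself.
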(event `self.ProjectileMovement.OnProjectileStop`
  (params (ImpactResult :type "HitResult Structure (by ref)"))
  (bind _outactors (`GameplayStatics.GetAllActorsOfClass` "/Script/Skyrunner.BaseEnemy"))
  (for _array_element _outactors
    (bind (_returnvalue_x _returnvalue_y _returnvalue_z) (`KismetMathLibrary.BreakVector` (- (`self.K2_GetActorLocation` _array_element) (`self.K2_GetActorLocation`))))
    (`Character.LaunchCharacter` _array_element (* (`KismetMathLibrary.Normal` (`KismetMathLibrary.MakeVector` _returnvalue_x _returnvalue_y (* _returnvalue_z (`self.ZMultiplier`)))) (`self.EnemyLaunchForce`)) true true))
  (`|SpawnActorFromClass` "/Game/Blueprints/Ability/BP_GravNadeInfluence.BP_GravNadeInfluence_C" (`KismetMathLibrary.MakeTransform` (`SceneComponent.K2_GetComponentLocation` (`self.Collision`)) (struct) (10.0 10.0 10.0)) "Undefined" "OverrideRootScale" null null)
  (`self.K2_DestroyActor`))

(fn `UserConstructionScript`)