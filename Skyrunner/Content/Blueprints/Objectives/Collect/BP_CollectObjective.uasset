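; Collect objective for Skyrunner that completes once all its spawned collectibles have been picked up.
; On BeginPlay it spawns a CollectibleClass actor at each of the game mode's ObjectiveSpawns, giving each a reference back to itself and counting them.
; OnPickupCollectible decrements the count, and IsComplete reports true at zero, guarded by IsStarted so it cannot pass before spawning finishes.
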(event `self.ReceiveBeginPlay`
  (`parent.ReceiveBeginPlay`)
  (bind _asskyrunner_game_mode_base_bp (cast `/Game/Blueprints/SkyrunnerGameModeBaseBP` (`GameplayStatics.GetGameMode`)))
  (for _array_element (`/Game/Blueprints/SkyrunnerGameModeBaseBP.ObjectiveSpawns` _asskyrunner_game_mode_base_bp)
    (bind _returnvalue (`|SpawnActorFromClass` (`self.CollectibleClass`) (`self.GetTransform` _array_element) "AlwaysSpawn" "OverrideRootScale" null null))
    (`/Engine/EditorBlueprintResources/StandardMacros.IsValid` _returnvalue
      (:`Is Valid`
        (set `/Game/Blueprints/Objectives/Collect/BP_Collectible.CollectObjective` self _returnvalue)
        (`/Engine/EditorBlueprintResources/StandardMacros.IncrementInt` (`self.AmountOfCollectibles`)))))
  (set `self.IsStarted` true))

(event `OnPickupCollectible`
  (`/Engine/EditorBlueprintResources/StandardMacros.DecrementInt` (`self.AmountOfCollectibles`)))

(fn `IsComplete`
  (returns (IsComplete :type Boolean))
  (return (and (<= (`self.AmountOfCollectibles`) 0) (`self.IsStarted`))))

(fn `UserConstructionScript`
  (`parent.UserConstructionScript`))