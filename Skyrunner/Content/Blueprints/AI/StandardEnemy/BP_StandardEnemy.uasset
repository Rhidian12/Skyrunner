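; BP_StandardEnemy is an AI enemy that spawns a gun, attaches it to its Arrow component and runs the BT_StandardEnemy behavior tree.
; On BeginPlay it also seeds the blackboard with the player character and the gun's rate of fire as AttackSpeed.
; Tick samples the player's location at a fixed interval into a rolling buffer, capped to a time window, dropping the oldest entry when full.
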(event `self.ReceiveBeginPlay`
  (bind _returnvalue (`|SpawnActorFromClass` "/Game/Blueprints/Guns/BP_StandardEnemyGun.BP_StandardEnemyGun_C" (`KismetMathLibrary.MakeTransform` (0.0 0.0 0.0)) "Undefined" "OverrideRootScale" null null))
  (bind _output_get (set `self.Gun` _returnvalue))
  (`self.K2_AttachToComponent` _output_get (`self.Arrow`) "None" "KeepRelative" "KeepRelative" "KeepRelative" true)
  (`AIController.RunBehaviorTree` (`AIBlueprintHelperLibrary.GetAIController` self) "/Game/Blueprints/AI/StandardEnemy/BT_StandardEnemy.BT_StandardEnemy")
  (`self.InitializeBlackboard`)
  (set `self.MaxBufferSize` (`KismetMathLibrary.FTrunc` (/ (`self.PositionBufferMaxTime`) (`self.PositionMaxTimer`)))))

(event `self.ReceiveTick`
  (params (DeltaSeconds :type "Float (single-precision)"))
  (bind _playerpositionbuffer (`self.PlayerPositionBuffer`))
  (bind _output_get (set `self.PositionTimer` (+ DeltaSeconds (`self.PositionTimer`))))
  (if (>= _output_get (`self.PositionMaxTimer`))
    (set `self.PositionTimer` 0.0)
    (if (>= (`KismetArrayLibrary.Array_Length` (`self.PlayerPositionBuffer`)) (`self.MaxBufferSize`))
      (`KismetArrayLibrary.Array_Remove` _playerpositionbuffer))
    (`KismetArrayLibrary.Array_Add` _playerpositionbuffer (`self.K2_GetActorLocation` (`self._Player`)))))

(fn `InitializeBlackboard`
  (locals (Player :type Name :default "Player") (_AttackSpeed :type Name :default "AttackSpeed") (PlayerBufferAverage :type Name :default "PlayerBufferAverage"))
  (bind _returnvalue (`AIBlueprintHelperLibrary.GetBlackboard` (`AIBlueprintHelperLibrary.GetAIController` self)))
  (bind _returnvalue_2 (`GameplayStatics.GetActorOfClass` "/Game/Blueprints/Player/PlayerCharacterBP.PlayerCharacterBP_C"))
  (`BlackboardComponent.SetValueAsObject` _returnvalue (`local.Player`) _returnvalue_2)
  (`BlackboardComponent.SetValueAsFloat` _returnvalue (`local._AttackSpeed`) (`BaseGun.RateOfFire` (`self.Gun`)))
  (set `self._Player` _returnvalue_2))

(fn `UserConstructionScript`)