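; BP_Sniper is an AI sniper enemy driven by the BT_Sniper behavior tree.
; On BeginPlay it spawns a BP_SniperGun, attaches it to GunPos, starts the tree and follows controller yaw.
; InitializeBlackboard then stores the player character and the gun's rate of fire, as AttackSpeed, in the blackboard.
; Damage and death events from BP_HealthComponent only print debug messages.
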(event `self.ReceiveBeginPlay`
  (bind _returnvalue (`|SpawnActorFromClass` "/Game/Blueprints/Guns/BP_SniperGun.BP_SniperGun_C" (`KismetMathLibrary.MakeTransform` (0.0 0.0 0.0)) "Undefined" "OverrideRootScale" null null))
  (bind _output_get (set `self.Gun` _returnvalue))
  (`self.K2_AttachToComponent` _returnvalue (`self.Gun Pos`) "None" "KeepRelative" "KeepRelative" "KeepRelative" true)
  (`self.K2_AttachToComponent` _output_get (`self.Gun Pos`) "None" "KeepRelative" "KeepRelative" "KeepRelative" true)
  (`AIController.RunBehaviorTree` (`AIBlueprintHelperLibrary.GetAIController` self) "/Game/Blueprints/AI/Sniper/BT_Sniper.BT_Sniper")
  (`self.InitializeBlackboard` (`BaseGun.RateOfFire` _returnvalue))
  (set `self.bUseControllerRotationYaw` true))

(event `self.BP_HealthComponent.OnDamage`
  (`KismetSystemLibrary.PrintString` "Sniper got hit"))

(event `self.BP_HealthComponent.OnDeath`
  (`KismetSystemLibrary.PrintString` "Sniper died!"))

(fn `InitializeBlackboard`
  (params (GunAttackSpeed :type "Float (double-precision)"))
  (locals (Player :type Name :default "Player") (AttackSpeed :type Name :default "AttackSpeed"))
  (bind _returnvalue (`AIBlueprintHelperLibrary.GetBlackboard` (`AIBlueprintHelperLibrary.GetAIController` self)))
  (bind _returnvalue_2 (`GameplayStatics.GetActorOfClass` "/Game/Blueprints/Player/PlayerCharacterBP.PlayerCharacterBP_C"))
  (`BlackboardComponent.SetValueAsObject` _returnvalue (`local.Player`) _returnvalue_2)
  (`BlackboardComponent.SetValueAsFloat` _returnvalue (`local.AttackSpeed`) GunAttackSpeed))

(fn `UserConstructionScript`)